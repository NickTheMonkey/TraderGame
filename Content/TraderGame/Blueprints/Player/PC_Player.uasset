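; Player controller for a trading and building game, forwarding camera input to the pawn and routing trades through a replicated resources component.
; Buy/sell amounts scale with x10/x100 modifiers; holding the autotrade keys instead marks resources for timed buying or selling above a saved minimum.
; Building checks data-table costs, moves a timer-driven preview box by cursor trace, then server-spawns BP_Building on click and deducts resources, optionally repeating for multi-build.
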(event `self.ReceiveBeginPlay`
  ;[1 0 0.9934] begin play
  (bind _returnvalue (`|SpawnActorFromClass` "/Game/TraderGame/Blueprints/Builds/Emptybox/BP_EmptyBox.BP_EmptyBox_C" (`KismetMathLibrary.MakeTransform` (0.0 0.0 -200.0)) "Undefined" "OverrideRootScale" null null))
  (set `self.BuildEmptybox` _returnvalue)
  (bind _returnvalue_2 (`KismetSystemLibrary.K2_SetTimerDelegate` (`|CreateDelegate` :!event `Autotrade`) 1.0 true))
  (set `self.Timer_Autotrade` _returnvalue_2))

(event `InputAction|Autotrade_CtrlShift`
  (params (Key :type "Key Structure"))
  ;[1 1 1] input
  (:`Pressed`
    (set `self.Auto_Trade` true :!label _label))
  (:`Released`
    (set `self.Auto_Trade` false :!label _label_2)))

(event `InputAxis|MoveCamera_Up`
  (params (AxisValue :type "Float (single-precision)"))
  (bind _returnvalue (`self.K2_GetPawn`))
  ;[1 1 1] input
  (`/Engine/EditorBlueprintResources/StandardMacros.IsValid` _returnvalue
    (:`Is Valid`
      (if (not (`KismetMathLibrary.NearlyEqual_FloatFloat` AxisValue 0.0 0.1))
        (message `/Game/TraderGame/Interfaces/BPI_Camera.Camera_Move_Up` _returnvalue AxisValue)))))

(event `InputAction|BuySell_Multiply_x10`
  (params (Key :type "Key Structure"))
  ;[1 1 1] input
  (:`Pressed`
    (set `self.BuySell_Multiply` 10.0))
  (:`Released`
    (set `self.BuySell_Multiply` 1.0)))

(event `InputAction|Autotrade_ShiftCtrl`
  (params (Key :type "Key Structure"))
  ;[1 1 1] input
  (:`Pressed`
    (goto _label))
  (:`Released`
    (goto _label_2)))

(event `InputAxis|MoveCamera_Right`
  (params (AxisValue :type "Float (single-precision)"))
  (bind _returnvalue (`self.K2_GetPawn`))
  ;[1 1 1] input
  (`/Engine/EditorBlueprintResources/StandardMacros.IsValid` _returnvalue
    (:`Is Valid`
      (if (not (`KismetMathLibrary.NearlyEqual_FloatFloat` AxisValue 0.0 0.1))
        (message `/Game/TraderGame/Interfaces/BPI_Camera.Camera_Move_Right` _returnvalue AxisValue)))))

(event `Autotrade`
  (bind _auto_trade_savedminimum_sell (`self.Auto_Trade_SavedMinimum_Sell`))
  (bind _cpp_acomp_resource (`self.CPP_AComp_Resource`))
  ;[1 1 1] autotrade
  (`|ExecutionSequence`
    (:`then_0`
      (for _array_element (`self.Auto_Trade_SavedMinimum_Buy`)
        (message `CPP_BPI_Resources.Resources_Buy` (`self.CPP_AComp_Resource`) _array_element 10.0)))
    (:`then_1`
      (bind _keys (`BlueprintMapLibrary.Map_Keys` _auto_trade_savedminimum_sell))
      (for _array_element_2 _keys
        (bind _amount (message `CPP_BPI_Resources.Resources_Get_Amount` _cpp_acomp_resource _array_element_2))
        (bind _returnvalue (- _amount (`BlueprintMapLibrary.Map_Find` _auto_trade_savedminimum_sell _array_element_2)))
        (if (> _returnvalue 0.0)
          (message `CPP_BPI_Resources.Resources_Sell` _cpp_acomp_resource _array_element_2 _returnvalue))))))

(event `InputAction|BuySell_Multiply_x100`
  (params (Key :type "Key Structure"))
  ;[1 1 1] input
  (:`Pressed`
    (set `self.BuySell_Multiply` 100.0))
  (:`Released`
    (set `self.BuySell_Multiply` 1.0)))

(event `ShowHide_BuildBox`
  (params (toShow :type Boolean))
  ;[1 1 1] build emptybox
  (`self.SetActorHiddenInGame` (`self.BuildEmptybox`) (not toShow))
  (if toShow
    (bind _returnvalue (`KismetSystemLibrary.K2_SetTimerDelegate` (`|CreateDelegate` :!event `BuildMouseTrace`) 0.05 true))
    (set `self.Timer_BuildEmptyboxLocation` _returnvalue)
    (else
      (`KismetSystemLibrary.K2_ClearAndInvalidateTimerHandle` (`self.Timer_BuildEmptyboxLocation`))
      (`self.K2_SetActorLocation` (`self.BuildEmptybox`) (0.0 0.0 0.0) false false))))

(event `InputAction|MultiBuild`
  (params (Key :type "Key Structure"))
  ;[1 1 1] input
  (:`Pressed`
    (set `self.isMultibuild_Pressed` true))
  (:`Released`
    (set `self.isMultibuild_Pressed` false)))

(event `InputAction|LMB`
  (params (Key :type "Key Structure"))
  (bind _returnvalue (`self.K2_GetActorLocation` (`self.BuildEmptybox`)))
  ;[1 1 1] input
  ;;[1 1 1] mouse
  (:`Pressed`
    (if (`KismetSystemLibrary.K2_IsTimerActiveHandle` (`self.Timer_BuildEmptyboxLocation`))
      (bind (_outhit _returnvalue_2) (`KismetSystemLibrary.LineTraceSingle` :`Start` (`KismetMathLibrary.MakeVector` (.x _returnvalue) (.y _returnvalue) (+ (.z _returnvalue) 400.0)) :`End` _returnvalue :`TraceChannel` "TraceTypeQuery1" :`DrawTime` 1.0))
      (bind (_bblockinghit _binitialoverlap _time _distance _location _impactpoint _normal _impactnormal _physmat _hitactor) (`GameplayStatics.BreakHitResult` _outhit))
      (if (!= (`GameplayStatics.GetObjectClass` _hitactor) "/Game/TraderGame/Blueprints/Builds/BP_Building.BP_Building_C")
        (`self.Server:Build_Spawn` (`KismetMathLibrary.SelectVector` _impactpoint _returnvalue _returnvalue_2) (`self.CurrentBuilding`) self)
        (message `CPP_BPI_Resources.Resources_Decrease_Array` (`self.CPP_AComp_Resource`) (`self.CurrentBuilding_ResourcesRequire`))
        (`self.ShowHide_BuildBox` (`self.isMultibuild_Pressed`))))))

(event `Build_NotEnoughResources`
  (`self.ShowHide_BuildBox` false))

(event `InputAction|RMB`
  (params (Key :type "Key Structure"))
  ;[1 1 1] input
  ;;[1 1 1] mouse
  (:`Pressed`
    (if (`KismetSystemLibrary.K2_IsTimerActiveHandle` (`self.Timer_BuildEmptyboxLocation`))
      (`self.ShowHide_BuildBox` false))))

(event `BuildMouseTrace`
  (bind (_bblockinghit _binitialoverlap _time _distance _location _impactpoint _normal _impactnormal _physmat _hitactor) (`GameplayStatics.BreakHitResult` (`self.GetHitResultUnderCursorByChannel` "TraceTypeQuery1")))
  (bind _returnvalue (`self.K2_GetActorLocation` _hitactor))
  (bind _returnvalue_2 (message `CPP_BPI_Resources.Resources_Get_Enough_Array` (`self.CPP_AComp_Resource`) (`self.CurrentBuilding_ResourcesRequire`)))
  (if _returnvalue_2
    (`/Engine/EditorBlueprintResources/StandardMacros.IsValid` _hitactor
      (:`Is Valid`
        (bind (_outhit _returnvalue_3) (`KismetSystemLibrary.LineTraceSingle` (`KismetMathLibrary.MakeVector` (.x _returnvalue) (.y _returnvalue) (+ (.z _returnvalue) 200.0)) _returnvalue "TraceTypeQuery1"))
        (if _returnvalue_3
          (`self.K2_SetActorLocation` (`self.BuildEmptybox`) (`.ImpactPoint` (`GameplayStatics.BreakHitResult` _outhit)) false false))))
    (else
      (`self.Build_NotEnoughResources`))))

(event `InputAxis|MouseWheel`
  (params (AxisValue :type "Float (single-precision)"))
  ;[1 1 1] input
  ;;[1 1 1] mouse
  (if (not (`KismetMathLibrary.NearlyEqual_FloatFloat` AxisValue 0.0 0.1))
    _))

(event `Server:Build_Spawn`
  (params (Location :type "Vector Structure") (CurrentBuilding :type "/Game/TraderGame/Data/ENUMS/E_Buildings Enum" :default "NewEnumerator0") (Owner :type "Controller Object Reference"))
  ;[1 1 1] Build spawn
  (`|SpawnActorFromClass` "/Game/TraderGame/Blueprints/Builds/BP_Building.BP_Building_C" (`KismetMathLibrary.MakeTransform` Location) "Undefined" "OverrideRootScale" Owner CurrentBuilding (`self.K2_GetPawn` Owner)))

(fn `Get_Resources_Component`
  (returns (Component :type "CPP_AComp_Resource Object Reference") (Success :type Boolean))
  (return (`self.CPP_AComp_Resource`) true))

(fn `GetAutotrade`
  (returns (Auto_Trade_SavedMinimum_Sell :type "Map of ResourceType Enum to Float (double-precision)") (Auto_Trade_SavedMinimum_Buy :type "Array of ResourceType Enum"))
  (return (`self.Auto_Trade_SavedMinimum_Sell`) (`self.Auto_Trade_SavedMinimum_Buy`)))

(fn `Resources_Buy`
  (params (resType :type "ResourceType Enum (by ref)") (amount :type "Float (double-precision) (by ref)"))
  (returns (ReturnValue :type Boolean))
  (bind _auto_trade_savedminimum_sell (`self.Auto_Trade_SavedMinimum_Sell`))
  (bind _restype (`local.resType`))
  (bind _auto_trade_savedminimum_buy (`self.Auto_Trade_SavedMinimum_Buy`))
  (if (`self.Auto_Trade`)
    (if (`KismetArrayLibrary.Array_Contains` _auto_trade_savedminimum_buy _restype)
      (bind _returnvalue (`KismetArrayLibrary.Array_RemoveItem` _auto_trade_savedminimum_buy _restype))
      (return _returnvalue)
      (else
        (`KismetArrayLibrary.Array_Add` _auto_trade_savedminimum_buy _restype)
        (`|ExecutionSequence`
          (:`then_0`
            (if (`.ReturnValue` (`BlueprintMapLibrary.Map_Find` _auto_trade_savedminimum_sell _restype))
              (`BlueprintMapLibrary.Map_Remove` _auto_trade_savedminimum_sell _restype)))
          (:`then_1`
            (return false)))))
    (else
      (bind _returnvalue_2 (message `CPP_BPI_Resources.Resources_Buy` (`self.CPP_AComp_Resource`) (`local.resType`) (* (`local.amount`) (`self.BuySell_Multiply`))))
      (return _returnvalue_2))))

(fn `Resources_Sell`
  (params (resType :type "ResourceType Enum (by ref)") (amount :type "Float (double-precision) (by ref)"))
  (returns (ReturnValue :type Boolean))
  (bind _restype (`local.resType`))
  (bind _auto_trade_savedminimum_buy (`self.Auto_Trade_SavedMinimum_Buy`))
  (bind _auto_trade_savedminimum_sell (`self.Auto_Trade_SavedMinimum_Sell`))
  (if (`self.Auto_Trade`)
    (if (`.ReturnValue` (`BlueprintMapLibrary.Map_Find` _auto_trade_savedminimum_sell _restype))
      (bind _returnvalue (`BlueprintMapLibrary.Map_Remove` _auto_trade_savedminimum_sell _restype))
      (return _returnvalue)
      (else
        (bind _amount (message `CPP_BPI_Resources.Resources_Get_Amount` (`self.CPP_AComp_Resource`) _restype))
        (`BlueprintMapLibrary.Map_Add` _auto_trade_savedminimum_sell _restype _amount)
        (`|ExecutionSequence`
          (:`then_0`
            (if (`KismetArrayLibrary.Array_Contains` _auto_trade_savedminimum_buy _restype)
              (`KismetArrayLibrary.Array_RemoveItem` _auto_trade_savedminimum_buy _restype)))
          (:`then_1`
            (return false)))))
    (else
      (bind _returnvalue_2 (message `CPP_BPI_Resources.Resources_Sell` (`self.CPP_AComp_Resource`) (`local.resType`) (* (`local.amount`) (`self.BuySell_Multiply`))))
      (return _returnvalue_2))))

(fn `ShowBuildbox`
  (params (Building_OLD :type "/Game/TraderGame/Data/ENUMS/E_Buildings Enum" :default "NewEnumerator0") (Building :type "BuildingType Enum" :default "BT_Mill"))
  (returns (Result :type Boolean))
  (locals (l_HaveResources :type Boolean :default true))
  (bind _output_get (set `self.CurrentBuilding` Building_OLD))
  (`BlueprintMapLibrary.Map_Clear` (`self.CurrentBuilding_ResourcesRequire`))
  (`self.ShowHide_BuildBox` false)
  (bind _returnvalue (`|GetDataTableRow` "/Game/TraderGame/Data/DataTables/DT_BuildingResources.DT_BuildingResources" (`KismetStringLibrary.Conv_StringToName` (`KismetStringLibrary.Concat_StrStr` (`|GetEnumeratorNameAsString` _output_get) "1")))
    (:`then`
      (set `self.CurrentBuilding_ResourcesRequire` (`.Resources_5_F5F7D5344D744A6E281E06812E5874AD` (break `/Game/TraderGame/Data/DataTables/S_BuildingResources` _returnvalue)))
      (bind _returnvalue_2 (message `CPP_BPI_Resources.Resources_Get_Enough_Array` (`self.CPP_AComp_Resource`) (`self.CurrentBuilding_ResourcesRequire`)))
      (if _returnvalue_2
        (`self.ShowHide_BuildBox` true)
        (return true)
        (else
          (`self.Build_NotEnoughResources`)
          (return false))))
    (:`RowNotFound`
      (return false))))

(fn `UserConstructionScript`
  (bind _cpp_acomp_resource (`self.CPP_AComp_Resource`))
  (`ActorComponent.SetIsReplicated` _cpp_acomp_resource true)
  (`ActorComponent.SetComponentTickEnabled` _cpp_acomp_resource false))