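; BP_Player is the player Blueprint, providing horizontal camera scrolling.
; The CameraMoveUp and CameraMoveRight axis events offset the actor along the control rotation's yaw, with the right axis turned 90 degrees from forward.
; Each offset scales by the axis value and ScrollSpeed, without sweep or delta-time scaling.
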(event `/Game/TraderGame/Interfaces/BPI_Camera.Camera_Move_Up`
  (params (Axis :type "Float (single-precision)"))
  (`self.K2_AddActorWorldOffset` (* (`KismetMathLibrary.Conv_RotatorToVector` (`KismetMathLibrary.MakeRotator` 0.0 0.0 (.yaw (`self.GetControlRotation`)))) (* Axis (`self.ScrollSpeed`)))))

(event `/Game/TraderGame/Interfaces/BPI_Camera.Camera_Move_Right`
  (params (Axis :type "Float (single-precision)"))
  (`self.K2_AddActorWorldOffset` (* (`KismetMathLibrary.Conv_RotatorToVector` (`KismetMathLibrary.MakeRotator` 0.0 0.0 (+ (.yaw (`self.GetControlRotation`)) 90.0))) (* Axis (`self.ScrollSpeed`)))))

(fn `UserConstructionScript`)