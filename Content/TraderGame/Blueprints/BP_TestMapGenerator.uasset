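; BP_TestMapGenerator is a test actor that builds a random tile map and spawns it as actors on BeginPlay.
; It clears old tiles, fills TestMap with tile IDs from seeded random streams, then spawns each ID's class from CurrentDA.
; Odd columns shift half a step, giving a staggered hex-style grid; lookup strides by Width, assuming square maps.
; SetMap only stores the map; Regenerate_Map is empty and the delayed rebuild is disconnected.
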(event `self.ReceiveTick`
  (params (DeltaSeconds :type "Float (single-precision)")))

(event `self.ReceiveBeginPlay`
  (bind (_width _height _tiles) (break `GameMap` (`self.TestMap`)))
  (bind (_width_2 _height_2 _tiles_2) (break `GameMap` (`self.TestMap`)))
  (bind _returnvalue (`KismetMathLibrary.Conv_ByteToInt` _width))
  (bind _returnvalue_2 (- (`KismetMathLibrary.Conv_ByteToInt` _width_2) 1))
  (for _array_element (`self.NewVar_2`)
    (`/Engine/EditorBlueprintResources/StandardMacros.IsValid` _array_element
      (:`Is Valid`
        (`self.K2_DestroyActor` _array_element))))
  (`/Engine/EditorBlueprintResources/StandardMacros.IncrementInt` (`self.NewVar_0`)
    (:`  `
      (`KismetArrayLibrary.Array_Clear` (`.Tiles` (break `GameMap` (`self.TestMap`))))
      (for _index (range (+ _returnvalue_2 1))
        (for _index_2 (range (`KismetMathLibrary.Conv_ByteToInt` _height_2))
          (`KismetArrayLibrary.Array_Add` _tiles_2 (`KismetMathLibrary.RandomIntegerInRangeFromStream` 1 3 (`KismetMathLibrary.MakeRandomStream` (* _index _index_2 (* (`self.NewVar_0`) 1) (- _returnvalue_2 _index_2)))))))
      (for _index_3 (range _returnvalue)
        (for _index_4 (range (`KismetMathLibrary.Conv_ByteToInt` _height))
          (bind _output (`|GetArrayItem` _tiles (+ _index_4 (* _index_3 _returnvalue))))
          (bind _returnvalue_3 (* _index_3 85.0))
          (bind _returnvalue_4 (* _index_4 90.0))
          (bind _returnvalue_5 (`|SpawnActorFromClass` (`DA_TilesMeshKeys.GetTileType` (`self.CurrentDA`) _output) (`KismetMathLibrary.MakeTransform` (+ (`KismetMathLibrary.SelectVector` (`KismetMathLibrary.MakeVector` _returnvalue_3 _returnvalue_4) (`KismetMathLibrary.MakeVector` _returnvalue_3 (+ _returnvalue_4 (* 90.0 0.5))) (== (mod _index_3 2) 0)) (`self.K2_GetActorLocation`)) (struct) (1.0 1.0 1.0)) "Undefined" "OverrideRootScale" null _output null))
          (`KismetArrayLibrary.Array_Add` (`self.NewVar_2`) _returnvalue_5))))))

(event `SetMap`
  (params (TestMap :type "GameMap Structure"))
  (set `self.TestMap` TestMap))

(event `Regenerate_Map`)

(fn `UserConstructionScript`)